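; Second-player pawn that moves on world X/Y and carries items between desks, with combining of ingredients.
; Tick lerps the Cube's rotation toward the UpDown/LeftRight input direction and sphere-traces forward from it.
; On PickUp/Drow2, DeskFunctions uses the traced BP_Desk to pick up or place an item by reattaching it.
; When both hand and desk are full, it calls Combine on the desk's BP_ingredient.
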(event EventTick
  (params (DeltaSeconds :type Float%20%28single-precision%29))
  (bind _cube (Variables|Default|GetCube))
  (bind _returnvalue (Transformation|GetWorldLocation _cube))
  (if (or (!= (Input|AxisValues|GetUpDown) 0.0) (!= 0.0 (Input|AxisValues|GetLeftRight)))
    ;[1 1 1] Set Wanted Dir
    (Variables|Default|Setdirection (Math|Vector|MakeVector (Input|AxisValues|GetUpDown) (Input|AxisValues|GetLeftRight) 0.0))
    (Transformation|SetWorldRotation (Variables|Default|GetCube) (Math|Rotator|Lerp(Rotator) (Transformation|GetWorldRotation (Variables|Default|GetCube)) (Math|Conversions|RotationFromXVector (Variables|Default|Getdirection)) (* DeltaSeconds (Variables|Default|GetRotationSpeed)) true) false false))
  (bind _outhit (Collision|SphereTraceByChannel _returnvalue (+ _returnvalue (* (Math|Vector|GetForwardVector _cube) (Variables|Default|GetReach))) (Variables|Default|GetRadius) "TraceTypeQuery1" false 0 "None")))

(event Input|ActionEvents|InputActionPickUp/Drow2
  (params (Key :type Key%20Structure))
  (:Pressed
    (CallFunction|DeskFunctions (.HitActor (Collision|BreakHitResult (stale EventTick _outhit))))))

(event Input|AxisEvents|InputAxisUpDown2
  (params (AxisValue :type Float%20%28single-precision%29))
  (Pawn|Input|AddMovementInput "1.000000,0.000000, 0" AxisValue false))

(event Input|AxisEvents|InputAxisLeftRight2
  (params (AxisValue :type Float%20%28single-precision%29))
  (Pawn|Input|AddMovementInput "0,1.000000, 0" AxisValue false))

(fn ConstructionScript)

(fn DeskFunctions
  (params (Desk :type Actor%20Object%20Reference))
  (bind _asbp_desk (Utilities|Casting|CastToBP_Desk Desk))
  (Utilities|IsValid (Variables|/Game/BP_Desk.BP_Desk_C|GetItem _asbp_desk)
    (:Is%20Valid
      (Utilities|IsValid (Variables|Default|GetHoldingItem)
        (:Is%20Valid
          ;[1 1 1] Possible Boxes combinations
          (bind _asbp_ingredient (Utilities|Casting|CastToBP_ingredient (Variables|/Game/BP_Desk.BP_Desk_C|GetItem _asbp_desk)))
          (Default|Combine _asbp_ingredient (Variables|Default|GetHoldingItem) 0 self))
        (:Is%20Not%20Valid
          ;[1 1 1] Pick up from desk
          (Transformation|DetachFromActor (Variables|/Game/BP_Desk.BP_Desk_C|GetItem _asbp_desk) "KeepWorld" "KeepWorld" "KeepWorld")
          (bind _output_get (Variables|Default|SetHoldingItem (Variables|/Game/BP_Desk.BP_Desk_C|GetItem _asbp_desk)))
          (Transformation|AttachComponentToComponent _output_get (Variables|Default|GetHoldingLocation) "None" "SnapToTarget" "KeepWorld" "KeepWorld" true)
          (Variables|/Game/BP_Desk.BP_Desk_C|SetItem _asbp_desk 0))))
    (:Is%20Not%20Valid
      (Utilities|IsValid (Variables|Default|GetHoldingItem)
        (:Is%20Valid
          (Transformation|DetachFromActor (Variables|Default|GetHoldingItem) "KeepWorld" "KeepWorld" "KeepWorld")
          (Transformation|AttachComponentToComponent (Variables|Default|GetHoldingItem) (Variables|/Game/BP_Desk.BP_Desk_C|GetItemLocation _asbp_desk) "None" "SnapToTarget" "KeepWorld" "KeepWorld" true)
          (Variables|/Game/BP_Desk.BP_Desk_C|SetItem _asbp_desk (Variables|Default|GetHoldingItem))
          (Variables|Default|SetHoldingItem 0))))))